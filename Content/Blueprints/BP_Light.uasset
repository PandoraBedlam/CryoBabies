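; Light actor that switches between a bright white powered look and a dim red unpowered look, following its PowerSource.
; The construction script creates a dynamic M_Emissive material on the Cylinder, so its color changes alongside the PointLight's color and intensity.
; BeginPlay binds to the PowerSource's OnPoweredChanged and applies the powered look without checking the current state; later events switch between the two looks.
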(event `self.ReceiveBeginPlay`
  (bind _pointlight (`self.PointLight`))
  (add `CBMachine.OnPoweredChanged` (`self.PowerSource`) (delegate `OnPoweredChanged_Event`))
  (`MaterialInstanceDynamic.SetVectorParameterValue` (`self.Material`) "Color" (struct :`R` 2.0 :`G` 2.0 :`B` 2.0 :`A` 1.0) :!label _label)
  (`LightComponent.SetIntensity` _pointlight 3000.0)
  (`LightComponent.SetLightColor` _pointlight (struct :`R` 1.0 :`G` 1.0 :`B` 1.0 :`A` 1.0) true))

(event `OnPoweredChanged_Event`
  (params (bIsPowered :type Boolean))
  (bind _pointlight (`self.PointLight`))
  (if bIsPowered
    (goto _label)
    (else
      (`MaterialInstanceDynamic.SetVectorParameterValue` (`self.Material`) "Color" (struct :`R` 0.2 :`A` 1.0))
      (`LightComponent.SetIntensity` _pointlight 500.0)
      (`LightComponent.SetLightColor` _pointlight (struct :`R` 0.2 :`A` 1.0) true))))

(fn `UserConstructionScript`
  (bind _returnvalue (`PrimitiveComponent.CreateDynamicMaterialInstance` (`self.Cylinder`) 0 "/Game/Art/Materials/M_Emissive.M_Emissive" "None"))
  (set `self.Material` _returnvalue))