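; Base machine Blueprint that takes a battery from whoever interacts with it.
; On Interact, a held BP_CBBattery is dropped by the interactor and force-added through AddBattery, while an empty-handed interactor triggers RemoveBattery.
; Other held pickups do nothing, and the battery and power logic itself is not defined in these graphs.
; Tick prints ChargeAmount and IsPowered on screen as debug output.
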(event `self.ReceiveTick`
  (params (DeltaSeconds :type "Float (single-precision)"))
  (`KismetSystemLibrary.PrintString` (`KismetStringLibrary.Conv_DoubleToString` (`self.ChargeAmount`)) true false (struct :`R` 1.0 :`G` 0.814822 :`A` 1.0) 0.0)
  (`KismetSystemLibrary.PrintString` (`KismetStringLibrary.Conv_BoolToString` (`self.bIsPowered`)) true true (struct :`R` 1.0 :`A` 1.0) 0.0))

(event `self.OnInteract`)

(event `self.Interact`
  (params (Interactor :type "CBCharacter Object Reference") (bIsInteracting :type Boolean))
  (bind _returnvalue (`CBCharacter.GetPickup` Interactor))
  (if (`KismetSystemLibrary.IsValid` _returnvalue)
    (bind _asbp_cbbattery (cast `/Game/Blueprints/BP_CBBattery` _returnvalue))
    (if (`KismetSystemLibrary.IsValid` _asbp_cbbattery)
      (`CBCharacter.DropPickup` Interactor)
      (`self.AddBattery` _asbp_cbbattery true))
    (else
      (`self.RemoveBattery`))))

(fn `UserConstructionScript`)