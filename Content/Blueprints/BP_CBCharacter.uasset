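; Player character Blueprint that gives its mesh a random colour and sets up proximity-style voice chat.
; BeginPlay tunes mic thresholds and gain through console commands, while InitializeVoiceChat adds a VOIP talker, retrying until PlayerState is valid before registering it with camera-attached attenuation and effects.
; Tick prints the voice level, and holding C enables loopback for testing.
; The colour is set locally without replication, flagged as a TODO.
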(event `self.ReceiveBeginPlay`
  (bind _mesh (`self.Mesh`))
  ;[1 0.15 0.15 0.5] Make this replicate correctly and C++
  (bind _returnvalue (`PrimitiveComponent.CreateDynamicMaterialInstance` _mesh 0 (`PrimitiveComponent.GetMaterial` _mesh 0) "None"))
  (`MaterialInstanceDynamic.SetVectorParameterValue` _returnvalue "BaseColour" (`KismetMathLibrary.MakeColor` (`KismetMathLibrary.RandomFloat`) (`KismetMathLibrary.RandomFloat`) (`KismetMathLibrary.RandomFloat`)))
  (`self.InitializeVoiceChat`)
  ; VoIP blueprint Logic (Maybe move the commands to c++)
  (`VOIPStatics.SetMicThreshold` -20.0)
  ;;[1 0.15 0.15 0.5] Todo: Make these sliders from 0 to 0.04
  (`KismetSystemLibrary.ExecuteConsoleCommand` "voice.SilenceDetectionThreshold 0.001" null)
  (`KismetSystemLibrary.ExecuteConsoleCommand` "voice.MicNoiseGateThreshold 0.001" null)
  (`KismetSystemLibrary.ExecuteConsoleCommand` "voice.MicInputGain 3" null)
  (`KismetSystemLibrary.ExecuteConsoleCommand` "ToggleSpeaking 1" null))

(event `Key|C`
  (params (Key :type "Key Structure"))
  ; Playback VOIP to self for testing
  (:`Pressed`
    (`KismetSystemLibrary.ExecuteConsoleCommand` "OSS.VoiceLoopback 1" null))
  (:`Released`
    (`KismetSystemLibrary.ExecuteConsoleCommand` "OSS.VoiceLoopback 0" null)))

(event `self.ReceiveTick`
  (params (DeltaSeconds :type "Float (single-precision)"))
  (bind _returnvalue (`VOIPTalker.GetVoiceLevel` (`self.VOIPRef`)))
  (`KismetSystemLibrary.PrintString` (`KismetStringLibrary.Conv_DoubleToString` _returnvalue) true true (struct :`G` 0.66 :`B` 1.0 :`A` 1.0) DeltaSeconds))

(event `InitializeVoiceChat`
  (bind _returnvalue (`AddComponent|NODE_AddVOIPTalker-1`))
  (set `self.VOIPRef` _returnvalue)
  (`/Engine/EditorBlueprintResources/StandardMacros.IsValid` (`self.PlayerState`) :!label _label
    (:`Is Valid`
      (`VOIPTalker.RegisterWithPlayerState` (`self.VOIPRef`) (`self.PlayerState`))
      (`VOIPStatics.SetMicThreshold` -1.0)
      (set `VOIPTalker.Settings` (make `VoiceSettings` (`self.CameraComponent`) "/Game/Audio/VOIP/SA_VOIP.SA_VOIP" "/Game/Audio/VOIP/SEPC_VOIP.SEPC_VOIP") (`self.VOIPRef`))
      (`KismetSystemLibrary.ExecuteConsoleCommand` "ToggleSpeaking 1" null))
    (:`Is Not Valid`
      (`KismetSystemLibrary.RetriggerableDelay` 0.2)
      (goto _label))))

(fn `UserConstructionScript`)