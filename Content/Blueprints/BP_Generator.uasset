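; BP_Generator is a generator that holds inserted batteries and tracks its own charge amount.
; While its charge is above zero, Tick picks the first inserted battery below maximum and lowers that battery's charge at the drain speed.
; It then adds the battery's shortfall from maximum, computed with a further drain step, to the generator's charge, clamped to its capacity.
; Full batteries are skipped.
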(event `self.ReceiveActorBeginOverlap`
  (params (OtherActor :type "Actor Object Reference"))
  (`parent.ReceiveActorBeginOverlap` OtherActor))

(event `self.ReceiveTick`
  (params (DeltaSeconds :type "Float (single-precision)"))
  (bind _output_get (set `self.Delta Seconds` DeltaSeconds))
  (`parent.ReceiveTick` _output_get)
  (if (> (`self.ChargeAmount`) 0.0)
    (for _array_element (`self.InsertedBatteries`)
      (bind _chargeamount (`CBBattery.ChargeAmount` _array_element))
      (bind _maxchargeamount (`CBBattery.MaxChargeAmount` _array_element))
      (if (< _chargeamount _maxchargeamount)
        (bind _returnvalue (`KismetMathLibrary.FClamp` (- _chargeamount (* (`self.ChargeDrainSpeed`) (`self.Delta Seconds`))) 0.0 _maxchargeamount))
        (set `CBBattery.ChargeAmount` _returnvalue _array_element)
        (set `self.ChargeAmount` (`KismetMathLibrary.FClamp` (+ (- (`CBBattery.MaxChargeAmount` _array_element) _returnvalue) (`self.ChargeAmount`)) 0.0 (`self.MaxCharge`)))
        (break)))))

(fn `UserConstructionScript`
  (`parent.UserConstructionScript`))