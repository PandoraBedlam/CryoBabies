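; BP_Machine is a machine that holds a charge and refills it from the batteries inserted into it.
; Each tick while below max, it moves charge at a drain rate from the first non-empty battery only, clamping both values.
; A dynamic emissive material on its sphere, created in the construction script, shows green while it has charge and red when empty.
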(event `self.ReceiveActorBeginOverlap`
  (params (OtherActor :type "Actor Object Reference"))
  (`parent.ReceiveActorBeginOverlap` OtherActor))

(event `self.ReceiveTick`
  (params (DeltaSeconds :type "Float (single-precision)"))
  (bind _lightmaterial (`self.LightMaterial`))
  (bind _output_get (set `self.Delta Seconds` DeltaSeconds))
  (`parent.ReceiveTick` _output_get)
  (if (> (`self.ChargeAmount`) 0.0)
    (`MaterialInstanceDynamic.SetVectorParameterValue` _lightmaterial "Color" (struct :`G` 0.5 :`A` 1.0))
    (else
      (`MaterialInstanceDynamic.SetVectorParameterValue` _lightmaterial "Color" (struct :`R` 0.5 :`A` 1.0))))
  (if (< (`self.ChargeAmount`) (`self.MaxCharge`))
    (for _array_element (`self.InsertedBatteries`)
      (bind _chargeamount (`CBBattery.ChargeAmount` _array_element))
      (if (> _chargeamount 0.0)
        (set `CBBattery.ChargeAmount` (`KismetMathLibrary.FClamp` (- _chargeamount (* (`self.BatteryDrainRate`) (`self.Delta Seconds`))) 0.0 (`CBBattery.MaxChargeAmount` _array_element)) _array_element)
        (set `self.ChargeAmount` (`KismetMathLibrary.FClamp` (+ (`self.ChargeAmount`) (* (`self.BatteryDrainRate`) (`self.Delta Seconds`))) 0.0 (`self.MaxCharge`)))
        (break)))))

(fn `UserConstructionScript`
  (`parent.UserConstructionScript`)
  (bind _returnvalue (`PrimitiveComponent.CreateDynamicMaterialInstance` (`self.Sphere`) 0 "/Game/Art/Materials/M_Emissive.M_Emissive" "None"))
  (set `self.LightMaterial` _returnvalue))